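; BP_BreakableDoor is a breakable door interactable with hooks for damage, kill, opening, falling and collision toggling.
; BeginPlay, construction, damage and kill effects, gate opening, forced opening and collision toggling only forward to the parent implementation.
; Fall, destroy, open-door, door-state replication and timeline handlers are empty here, and GetGroundOffset returns zero.
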(event `self.ReceiveBeginPlay`
  (`parent.ReceiveBeginPlay`))

(event `KilledTimeline__FinishedFunc`)

(event `KilledTimeline__UpdateFunc`)

(event `KilledTimeline__NewTrack_1__EventFunc`)

(event `DamageTimeline__FinishedFunc`)

(event `DamageTimeline__UpdateFunc`)

(event `Timeline_0__FinishedFunc`)

(event `Timeline_0__UpdateFunc`)

(event `self.KilledFx`
  (`parent.KilledFx`))

(event `self.DamageFx`
  (`parent.DamageFx`))

(event `self.ForceOpened`
  (params (OpenGateDirection :type Byte))
  (`parent.ForceOpened` OpenGateDirection))

(event `self.OpenGate`
  (params (OpenGateDirection :type Byte))
  (`parent.OpenGate` OpenGateDirection))

(event `TriggerFall`
  (params (Forward :type Boolean)))

(event `DestroyDoor`)

(event `OpenDoor`
  (params (Open :type Boolean)))

(event `SetDoorOpened`)

(event `self.ToggleDoorCollision`
  (params (Enabled :type Boolean))
  (`parent.ToggleDoorCollision` Enabled))

(fn `GetGroundOffset`
  (params (Forward :type Boolean))
  (returns (` ` :type "Float (double-precision)"))
  (return 0.0))

(fn `OnRep_DoorState`)

(fn `UserConstructionScript`
  (`parent.UserConstructionScript`))