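; Breakable cheval de frise barricade actor for the Darkforest set, a child of a parent Blueprint that supplies its behavior.
; BeginPlay, overlaps, breakable state changes, mesh collision removal and construction only forward to the parent.
; Ragdoll attach and detach, kill FX and SetBroken events are empty, Tick is disabled, and the ragdoll attach params function returns without setting values.
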(event `self.ReceiveBeginPlay`
  (`parent.ReceiveBeginPlay`))

(event `self.ReceiveActorBeginOverlap`
  (params (OtherActor :type "Actor Object Reference"))
  (`parent.ReceiveActorBeginOverlap` OtherActor))

(event `OnRagdollAttach`
  (params (Character :type "TBLCharacter Object Reference")))

(event `OnRagdollDetach`
  (params (Character :type "TBLCharacter Object Reference")))

(event `KilledFx_1`)

(event `self.ReceiveActorEndOverlap`
  (params (OtherActor :type "Actor Object Reference"))
  (`parent.ReceiveActorEndOverlap` OtherActor))

(event `self.BreakableStateChanged`
  (params (BreakableState :type Byte))
  (`parent.BreakableStateChanged` BreakableState))

(event `SetBroken`)

(event `self.RemoveCollisionOnMeshes`
  (`parent.RemoveCollisionOnMeshes`))

(fn `GetAttachRagdollParams`
  (params (Character :type "TBLCharacter Object Reference") (DamageEvent :type " Structure (by ref)"))
  (returns (AttachRagdollParams :type " Structure"))
  (return))

(fn `UserConstructionScript`
  (`parent.UserConstructionScript`))