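; Breakable Darkforest cheval-de-frise barricade variant (02B), built as a child of a parent breakable Blueprint.
; Construction, overlap, kill FX and breakable state changes only forward to the parent, and Tick is disabled.
; Ragdoll attach and detach events and SetBroken are empty stubs, and GetAttachRagdollParams returns without setting values, so the graphs add no logic of their own.
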(event `self.ReceiveBeginPlay`
  (`parent.ReceiveBeginPlay`))

(event `self.ReceiveActorBeginOverlap`
  (params (OtherActor :type "Actor Object Reference"))
  (`parent.ReceiveActorBeginOverlap` OtherActor))

(event `OnRagdollAttach`
  (params (Character :type "TBLCharacter Object Reference")))

(event `OnRagdollDetach`
  (params (Character :type "TBLCharacter Object Reference")))

(event `self.KilledFx`
  (params (DamageTakenEvent :type "DamageTakenEvent Structure (by ref)"))
  (`parent.KilledFx` (struct)))

(event `self.ReceiveActorEndOverlap`
  (params (OtherActor :type "Actor Object Reference"))
  (`parent.ReceiveActorEndOverlap` OtherActor))

(event `self.BreakableStateChanged`
  (params (BreakableState :type "/Game/Interactables/Objectives/BreakableGate/BreakableState Enum" :default "NewEnumerator0"))
  (`parent.BreakableStateChanged` BreakableState))

(event `SetBroken`)

(fn `GetAttachRagdollParams`
  (params (Character :type "TBLCharacter Object Reference") (DamageEvent :type "DeathDamageTakenEvent Structure (by ref)"))
  (returns (AttachRagdollParams :type "AttachRagdollParams Structure"))
  (return))

(fn `UserConstructionScript`
  (`parent.UserConstructionScript`))