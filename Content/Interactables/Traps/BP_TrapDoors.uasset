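; BP_TrapDoors is a trap door interactable, a child Blueprint that adds no logic of its own in its graphs.
; BeginPlay, the construction script and the simple-door gate opened and closed events only forward to the parent.
; The gate close, closing enable and disable, permanent open and trigger hit events are empty stubs with no parent call.
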(event `self.ReceiveBeginPlay`
  (`parent.ReceiveBeginPlay`))

(event `GateClose`)

(event `self.OnGateClosedEvent_SimpleDoor`
  (params (Value :type "Float (single-precision)"))
  (`parent.OnGateClosedEvent_SimpleDoor` Value))

(event `self.OnGateOpenedEvent_SimpleDoor`
  (params (Value :type "Float (single-precision)"))
  (`parent.OnGateOpenedEvent_SimpleDoor` Value))

(event `DisableGateClosing`)

(event `PermanentlyOpenDoor`
  (params (Open :type Boolean)))

(event `EnableGateClosing`)

(event `TriggerHit`)

(fn `UserConstructionScript`
  (`parent.UserConstructionScript`))