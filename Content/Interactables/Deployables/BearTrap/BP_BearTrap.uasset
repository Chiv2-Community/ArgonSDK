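; BP_BearTrap is a deployable bear trap Blueprint, built on a parent that supplies constructable behavior such as DestroyConstructable.
; BeginPlay, construction and destruction only forward to the parent, while overlap and tick are disabled.
; Trap triggering, damage application and ragdoll attach and detach hooks are empty stubs, and GetAttachRagdollParams returns without any logic.
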(event `self.ReceiveBeginPlay`
  (`parent.ReceiveBeginPlay`))

(event `AttachRagdollInterface.OnRagdollAttach`
  (params (Character :type "TBLCharacter Object Reference")))

(event `AttachRagdollInterface.OnRagdollDetach`
  (params (Character :type "TBLCharacter Object Reference")))

(event `self.DestroyConstructable`
  (`parent.DestroyConstructable`))

(event `ApplyDamage`)

(fn `GetAttachRagdollParams`
  (params (Character :type "TBLCharacter Object Reference") (DamageEvent :type "DeathDamageTakenEvent Structure (by ref)"))
  (returns (AttachRagdollParams :type "AttachRagdollParams Structure"))
  (return))

(fn `TriggerTrap`)

(fn `UserConstructionScript`
  (`parent.UserConstructionScript`))