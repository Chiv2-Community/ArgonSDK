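; Breakable pavise shield deployable, a Blueprint that adds almost no logic of its own.
; BeginPlay, construction, ForceBrokenState and KilledFx forward to the parent class.
; Team update, FFA material, lifespan reset, self-destroy, timeline and load events have empty bodies, and GetGroundOffset returns zero.
; Tick and overlap are disabled.
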(event `self.ReceiveBeginPlay`
  (`parent.ReceiveBeginPlay`))

(event `Timeline_0__FinishedFunc`)

(event `Timeline_0__UpdateFunc`)

(event `Timeline_0__NewTrack_1__EventFunc`)

(event `OnLoaded_DEBF5ABE4C7A2C6A44D871B4C01A8397`
  (params (Loaded :type "Object Object Reference")))

(event `KilledFx_1`)

(event `ApplyFFAMaterial`
  (params (Material :type "MaterialInterface Object Reference")))

(event `self.ForceBrokenState`
  (`parent.ForceBrokenState`))

(event `ResetLifespanTimer`)

(event `DestroySelf`)

(event `self.KilledFx`
  (params (DamageTakenEvent :type "DamageTakenEvent Structure (by ref)"))
  (`parent.KilledFx` DamageTakenEvent))

(fn `GetGroundOffset`
  (params (Forward :type Boolean))
  (returns (` ` :type "Float (double-precision)"))
  (return 0.0))

(fn `UpdateTeam`)

(fn `UserConstructionScript`
  (`parent.UserConstructionScript`))