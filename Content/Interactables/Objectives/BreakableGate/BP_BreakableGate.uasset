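; BP_BreakableGate is a breakable gate objective interactable that can be opened, forced open or forced into a broken state.
; It is a thin child Blueprint: damage effects, opening, broken-state and construction logic all defer to the parent class.
; Its timeline callbacks and inward, outward and reverse timeline control events are empty stubs in this graph.
; BeginPlay, overlap and Tick are disabled.
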(event `Timeline_1__FinishedFunc`)

(event `Timeline_1__UpdateFunc`)

(event `Timeline_0_0__FinishedFunc`)

(event `Timeline_0_0__UpdateFunc`)

(event `Timeline_2__FinishedFunc`)

(event `Timeline_2__UpdateFunc`)

(event `Timeline_0__FinishedFunc`)

(event `Timeline_0__UpdateFunc`)

(event `self.DamageFx`
  (`parent.DamageFx`))

(event `self.ForceOpened`
  (params (OpenGateDirection :type Byte))
  (`parent.ForceOpened` OpenGateDirection))

(event `self.OpenGate`
  (params (OpenGateDirection :type Byte))
  (`parent.OpenGate` OpenGateDirection))

(event `self.ForceBrokenState`
  (`parent.ForceBrokenState`))

(event `SetInwardTimeline`
  (params (Time :type "Float (double-precision)")))

(event `SetOutwardTimeline`
  (params (Time :type "Float (double-precision)")))

(event `ReverseActiveTimeline`)

(event `ReverseInwardTimelime`)

(event `ReverseOutwardTimelime`)

(fn `UserConstructionScript`
  (`parent.UserConstructionScript`))