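; Breakable gate objective variant for the Coxwell Market exit, built as a child Blueprint of a shared gate class.
; BeginPlay, ForceOpened, OpenGate and the construction script only forward to the parent, which supplies the gate behavior.
; PlayDoorVFX has an empty body here, and two timelines have unconnected update and finished events.
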(event `self.ReceiveBeginPlay`
  (`parent.ReceiveBeginPlay`))

(event `Timeline_3__FinishedFunc`)

(event `Timeline_3__UpdateFunc`)

(event `Timeline_4__FinishedFunc`)

(event `Timeline_4__UpdateFunc`)

(event `/Game/Interactables/Objectives/BreakableGate/BP_BaseBreakableGate.ForceOpened`
  (params (OpenGateDirection :type "/Game/Interactables/Objectives/BreakableGate/GateDirection Enum" :default "NewEnumerator2"))
  (`parent.ForceOpened` OpenGateDirection))

(event `/Game/Interactables/Objectives/BreakableGate/BP_BaseBreakableGate.OpenGate`
  (params (OpenGateDirection :type "/Game/Interactables/Objectives/BreakableGate/GateDirection Enum" :default "NewEnumerator2"))
  (`parent.OpenGate` OpenGateDirection))

(fn `PlayDoorVFX`)

(fn `UserConstructionScript`
  (`parent.UserConstructionScript`))