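; BP_ConstructableRamp is a constructable ramp objective interactable that relies on its parent class for all construction behavior.
; BeginPlay, the construction script, and the construction stage and completion events only forward to the parent.
; Overlap and Tick are disabled, and a leftover timeline's update, finished and event-track handlers are empty.
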(event `self.ReceiveBeginPlay`
  (`parent.ReceiveBeginPlay`))

(event `Timeline_1__FinishedFunc`)

(event `Timeline_1__UpdateFunc`)

(event `Timeline_1__NewTrack_0__EventFunc`)

(event `self.OnConstructionCompleted_Event`
  (`parent.OnConstructionCompleted_Event`))

(event `self.OnConstruction_Event`
  (params (NewStage :type Integer) (PreviousStage :type Integer))
  (`parent.OnConstruction_Event` NewStage PreviousStage))

(fn `UserConstructionScript`
  (`parent.UserConstructionScript`))