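; Library variant of the constructable petard objective, a Blueprint child that inherits its construction and fuse behavior from its parent.
; BeginPlay, construction events, fuse start and stop, and the construction script only forward to parent implementations.
; Library-named fuse lit and defused events, a fuse destroyed event and two generic custom events are empty stubs, so this asset adds no logic of its own.
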(event `self.ReceiveBeginPlay`
  (`parent.ReceiveBeginPlay`))

(event `/Game/Interactables/Objectives/Constructables/BP_BaseConstructable.OnConstruction_Event`
  (params (NewStage :type Integer) (PreviousStage :type Integer))
  (`parent.OnConstruction_Event` NewStage PreviousStage))

(event `self.StartFuse`
  (`parent.StartFuse`))

(event `self.StopFuse`
  (`parent.StopFuse`))

(event `CustomEvent_1`
  (params (Value :type "Float (double-precision)")))

(event `CustomEvent`
  (params (Value :type "Float (double-precision)")))

(event `FuseLit_Event_Library`)

(event `FuseDefused_Event_Library`)

(event `FuseDestroyed_Event_0`)

(fn `UserConstructionScript`
  (`parent.UserConstructionScript`))