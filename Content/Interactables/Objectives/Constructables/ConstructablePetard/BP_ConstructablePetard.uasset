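; Constructable petard objective, with hooks for igniting and defusing a fuse, scoring the defuser and dealing explosion damage to characters in a cone.
; BeginPlay, construction events, the construction script and the next-stage check only forward to the parent class.
; The fuse, interactable, kill, scoring and damage graphs are empty stubs here, GetFuseTime returns zero, and Tick and overlap are disabled.
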(event `self.ReceiveBeginPlay`
  (`parent.ReceiveBeginPlay`))

(event `self.OnConstructionCompleted_Event`
  (`parent.OnConstructionCompleted_Event`))

(event `self.OnConstruction_Event`
  (params (NewStage :type Integer) (PreviousStage :type Integer))
  (`parent.OnConstruction_Event` NewStage PreviousStage))

(event `OnKilled_Event_0`
  (params (Event :type " Structure (by ref)")))

(event `CustomEvent_0`)

(event `UpdateInteractables`
  (params (`Enable Defuse` :type Boolean) (`Enable Ignite` :type Boolean)))

(event `StartFuse`)

(event `StopFuse`)

(event `GiveScoreToDefuser`
  (params (Target :type "Pawn Object Reference")))

(event `OnKilled_Event_BaseConstructablePetard`
  (params (Event :type "DeathDamageTakenEvent Structure (by ref)")))

(fn `ApplyExplosionDamageToCharactersInCone`
  (params (OverlappingActors :type "Array of Actor Object Reference (by ref)") (DamageCauser :type "Actor Object Reference")))

(fn `CanConstructNextStage`
  (returns (` ` :type Boolean))
  (return (`parent.CanConstructNextStage`)))

(fn `GetFuseTime`
  (returns (FuseTime :type "Float (double-precision)"))
  (return 0.0))

(fn `GetOverlappingCharacters`
  (returns (OutActors :type "Array of Actor Object Reference"))
  (return))

(fn `OnRep_IsFuseLit`)

(fn `UserConstructionScript`
  (`parent.UserConstructionScript`))