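; Spawner Blueprint for the freeable VIP objective, built as a stub with no gameplay logic of its own.
; Spawn animation and cinematic control events are empty, and the spawn location and max player count functions return only zero defaults.
; BeginPlay, overlap and Tick are disabled placeholders, and the construction script only calls its parent.
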(event `DoSpawnAnimation`
  (params (Character :type "TBLCharacter Object Reference")))

(event `Cinematics_StartAllowingControl`
  (params (Character :type "TBLCharacter Object Reference")))

(event `OnPlaySpawnAnimation`
  (params (Animation :type Name)))

(fn `GetMaxPlayerCount`
  (returns (ReturnValue :type Integer))
  (return 0))

(fn `GetSpawnLocationAndComponent`
  (params (Index :type Integer))
  (returns (OutTransform :type "Transform Structure") (SpawnRadius :type "Float (double-precision)") (SpawnHalfHeight :type "Float (double-precision)") (ReturnValue :type "SceneComponent Object Reference"))
  (return (struct) 0.0 0.0 null))

(fn `UserConstructionScript`
  (`parent.UserConstructionScript`))