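; Pushable, interactable drop zone for carryables in the capture point system, built as an LD variant whose behavior comes mostly from its parent class.
; BeginPlay, construction, drop zone activation and deactivation, and loaded count changes simply forward to the parent.
; ActivatePushable, the carryable capture handler, GrantPlayerScore and UpdateActorInfo are empty with no parent calls, so this Blueprint adds no logic of its own.
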(event `self.ReceiveBeginPlay`
  (`parent.ReceiveBeginPlay`))

(event `ActivatePushable`)

(event `PlayerCapturedCarryable_Event_0`
  (params (Team :type "TBLTeam Object Reference") (Player :type "TBLCharacter Object Reference") (Value :type "Float (double-precision)")))

(event `self.OnLoadedCountChanged`
  (`parent.OnLoadedCountChanged`))

(event `GrantPlayerScore`
  (params (Pawn :type "Pawn Object Reference")))

(event `self.ActivateDropZone`
  (`parent.ActivateDropZone`))

(event `self.DeactivateDropZone`
  (`parent.DeactivateDropZone`))

(event `UpdateActorInfo`)

(fn `UserConstructionScript`
  (`parent.UserConstructionScript`))