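; Environment spline tool actor that places meshes along a spline, with landscape snapping, deformation and painting.
; Function names indicate size-variant fitting with curve search and pinch checks, start and end caps, offsets and randomized transforms, output as spline mesh, static mesh or HISM instances.
; Editor-style events cover seed generation, surface snapping, terrain deform and paint, and layer checks.
; All graph bodies, including the construction script, are empty here.
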(event `Generate Seed`)

(event `Snap Spline to Surface`)

(event `Deform And Paint Terrain`)

(event `Deform Terrain`)

(event `Paint Terrain`)

(event `CheckLandscapeLayers`)

(fn `A Take Z of B`
  (params (A :type "Vector Structure") (B :type "Vector Structure"))
  (returns (`AXY-BZ` :type "Vector Structure"))
  (return (0.0 0.0 0.0)))

(fn `AddCapMesh`
  (params (Mesh :type "StaticMesh Object Reference") (CapOffset :type "Float (double-precision)") (CapTransformStart :type " Structure") (CapTransformEnd :type " Structure")))

(fn `AddErrors`
  (params (ErrorText :type String)))

(fn `AddTransformAtDistance`
  (params (SizeVariantIndex :type Integer) (Distance :type "Float (double-precision)")))

(fn `CenterpointSmooth`
  (params (Start :type "Transform Structure") (End :type "Transform Structure"))
  (returns (StartSmooth :type "Transform Structure"))
  (return))

(fn `CheckForZeroOffsets`
  (returns (MeshContainsZeroOffset :type Boolean))
  (return false))

(fn `CreateDistanceOffset`
  (params (Distance :type "Float (double-precision)"))
  (returns (Index :type Integer) (Offset :type "Float (double-precision)"))
  (return 0 0.0))

(fn `CreateEndCapTransforms`
  (params (StartLoc :type "Vector Structure")))

(fn `CreateHISMComponentsForVariants`
  (params (MeshVariants :type "Array of  Structure (by ref)"))
  (returns (`HISM Components` :type "Array of HierarchicalInstancedStaticMeshComponent Object Reference") (`Variant Probabilities` :type "Array of Float (double-precision)"))
  (return))

(fn `CreateMeshAlongSpline`
  (params (CurrentIndex :type Integer)))

(fn `CreateMeshInstances`
  (params (SizeVariant :type "Array of  Structure (by ref)")))

(fn `CreateStartCapTransforms`
  (returns (StartLoc :type "Vector Structure"))
  (return (0.0 0.0 0.0)))

(fn `CreateStaticMeshesForVariants`
  (params (MeshVariants :type "Array of  Structure (by ref)"))
  (returns (`Static Meshes` :type "Array of StaticMesh Object Reference") (`Variant Probabilities` :type "Array of Float (double-precision)"))
  (return))

(fn `CurveEndCheck`
  (params (LastEndPoint :type "Vector Structure") (Sizes :type "Array of Float (double-precision) (by ref)"))
  (returns (HitEnd :type Boolean))
  (return false))

(fn `CurveZProjection`
  (params (StartPoint :type "Vector Structure") (Endpoint :type "Vector Structure") (Iterations :type Integer))
  (returns (ProjectedEndpoint :type "Vector Structure"))
  (return (0.0 0.0 0.0)))

(fn `FindLandscape`
  (params (AllowDebug :type Boolean))
  (returns (LandscapeSoft :type "Landscape Object Reference"))
  (return null))

(fn `GetDistanceAlongSplineForWorldLocation`
  (params (Spline :type "SplineComponent Object Reference") (Location :type "Vector Structure"))
  (returns (Distance :type "Float (double-precision)"))
  (return 0.0))

(fn `LandscapeLayer`
  (params (DeformationSettings :type " Structure")))

(fn `LocalOffset`
  (params (BasePosition :type "Vector Structure") (Direction :type "Vector Structure") (Offset :type "Vector Structure"))
  (returns (OffsetPosition :type "Vector Structure"))
  (return (0.0 0.0 0.0)))

(fn `OverrideMaterials`
  (params (`Target Mesh` :type "PrimitiveComponent Object Reference")))

(fn `RandomizeTransforms`
  (params (BaseTransform :type "Transform Structure") (TransformMin :type "Transform Structure") (TransformMax :type "Transform Structure"))
  (returns (Randomized :type "Transform Structure"))
  (return))

(fn `SaveSplineTransforms`)

(fn `SearchCurve`
  (params (StartLoc :type "Vector Structure") (ProjDistance :type "Float (double-precision)"))
  (returns (Rotation :type "Rotator Structure") (EndLoc :type "Vector Structure") (EndTan :type "Vector Structure") (EndRoll :type "Float (double-precision)"))
  (return (struct) (0.0 0.0 0.0) (0.0 0.0 0.0) 0.0))

(fn `SearchCurvePinch`
  (params (StartLocation :type "Vector Structure") (EndLocation :type "Vector Structure") (LastPointLocation :type "Vector Structure") (Offset :type "Float (double-precision)") (PinchRatios :type "Array of Float (double-precision) (by ref)") (ZRatio :type "Array of Float (double-precision) (by ref)") (CurrentIndex :type Integer))
  (returns (ShouldDivide :type Boolean))
  (return false))

(fn `Set Z 0`
  (params (A :type "Vector Structure"))
  (returns (`AZ-0` :type "Vector Structure"))
  (return (0.0 0.0 0.0)))

(fn `SetSplineOffset`
  (params (Offset :type "Vector2D Structure")))

(fn `SetSplineTransforms`
  (params (Transforms :type "Array of Vector Structure (by ref)")))

(fn `SnapSplineToTerrain`)

(fn `SnapTransformToTerrain`
  (params (Start :type "Transform Structure") (End :type "Transform Structure"))
  (returns (Snapped :type "Transform Structure") (SnappedTan :type "Vector Structure") (HitSuccess :type Boolean))
  (return (struct) (0.0 0.0 0.0) false))

(fn `SortMeshSizes`
  (params (Unsorted :type "Array of  Structure (by ref)") (ReverseOrder :type Boolean))
  (returns (Sorted :type "Array of  Structure"))
  (return))

(fn `SpawnHISMInstance`
  (params (Mesh :type "InstancedStaticMeshComponent Object Reference") (CurrentIndex :type Integer)))

(fn `SpawnSplineMeshInstance`
  (params (Mesh :type "StaticMesh Object Reference") (CurrentIndex :type Integer) (Offset :type "Float (double-precision)")))

(fn `SplineStretchToFit`
  (params (`Size Variants` :type "Array of Float (double-precision) (by ref)")))

(fn `TransformToLocal`
  (params (Location :type "Vector Structure"))
  (returns (LocalLocation :type "Vector Structure"))
  (return (0.0 0.0 0.0)))

(fn `TransformToWorld`
  (params (Location :type "Vector Structure"))
  (returns (WorldLocation :type "Vector Structure"))
  (return (0.0 0.0 0.0)))

(fn `UserConstructionScript`)

(fn `VisualizeLandscapeDeformation`)