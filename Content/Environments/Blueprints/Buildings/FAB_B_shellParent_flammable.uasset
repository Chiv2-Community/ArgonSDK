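; Parent Blueprint for flammable building shells, judging by its name, with no flammability logic in its graphs.
; BeginPlay and the construction script only call their parent versions, while overlap and Tick are disabled.
; The health-change event is an empty stub, and the HUD marker location and progress functions return zero.
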(event `self.ReceiveBeginPlay`
  (`parent.ReceiveBeginPlay`))

(event `OnStatHealthChanged`
  (params (Amount :type "Float (double-precision)") (Initiator :type "Actor Object Reference")))

(fn `GetHUDMarkerLocation`
  (params (PlayerController :type "PlayerController Object Reference"))
  (returns (ReturnValue :type "Vector Structure"))
  (return (0.0 0.0 0.0)))

(fn `GetHUDMarkerProgress`
  (params (PlayerController :type "PlayerController Object Reference"))
  (returns (ReturnValue :type "Float (double-precision)"))
  (return 0.0))

(fn `UserConstructionScript`
  (`parent.UserConstructionScript`))