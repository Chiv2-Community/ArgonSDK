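; BPF_Gameplay is a Blueprint function library of gameplay helpers for melee combat, with every body here a stub.
; Query functions cover player control, enemy checks, pawn states like downed, airborne, sprinting, mounted or parrying, and shove, jab and tackle identification.
; TBL-prefixed functions declare sphere actor lookup, pawn killing, and damage and crowd-control application, either single-target or by radius.
; All bodies are empty or return defaults, so only the signatures carry information.
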(fn `GetShoveInstigator`
  (params (Character :type "TBLCharacter Object Reference"))
  (returns (ShoveInstigator :type "Actor Object Reference"))
  (return null))

(fn `Is Shove Or Jab Or Headbutt Ability Spec`
  (params (` 1` :type "AbilitySpec Object Reference"))
  (returns (`  ` :type Boolean))
  (return false))

(fn `IsCharacterParryingWithShield`
  (params (Target :type "TBLCharacter Object Reference"))
  (returns (ReturnValue :type Boolean))
  (return false))

(fn `IsControllerPlayerControlled`
  (params (Controller :type "Controller Object Reference"))
  (returns (bReturnValue :type Boolean))
  (return false))

(fn `IsEnemy`
  (params (TestA :type "Actor Object Reference") (TestB :type "Actor Object Reference"))
  (returns (` ` :type Boolean))
  (return false))

(fn `IsInCrowdControlState`
  (params (Target :type "Actor Object Reference"))
  (returns (` ` :type Boolean))
  (return false))

(fn `IsInJabKnockback`
  (params (Character :type "TBLCharacter Object Reference"))
  (returns (` ` :type Boolean))
  (return false))

(fn `IsInShoveKnockback`
  (params (Character :type "TBLCharacter Object Reference"))
  (returns (` ` :type Boolean))
  (return false))

(fn `IsJabAttack`
  (params (DamageTakenEvent :type "DamageTakenEvent Structure (by ref)"))
  (returns (` ` :type Boolean))
  (return false))

(fn `IsMounted`
  (params (Actor :type "Actor Object Reference"))
  (returns (` ` :type Boolean))
  (return false))

(fn `IsObjectPlayerControlled`
  (params (Object :type "Object Object Reference"))
  (returns (bReturnValue :type Boolean))
  (return false))

(fn `IsPawnAirborne`
  (params (Target :type "Pawn Object Reference"))
  (returns (` ` :type Boolean))
  (return false))

(fn `IsPawnDowned`
  (params (Target :type "Pawn Object Reference"))
  (returns (` ` :type Boolean))
  (return false))

(fn `IsPawnInSpecialAttack`
  (params (Target :type "Pawn Object Reference"))
  (returns (` ` :type Boolean))
  (return false))

(fn `IsPawnInSprintAttack`
  (params (Target :type "Pawn Object Reference"))
  (returns (` ` :type Boolean))
  (return false))

(fn `IsPawnPlayerControlled`
  (params (Pawn :type "Pawn Object Reference"))
  (returns (bReturnValue :type Boolean))
  (return false))

(fn `IsPawnSprinting`
  (params (Target :type "Pawn Object Reference"))
  (returns (` ` :type Boolean))
  (return false))

(fn `IsPlayerControlled`
  (params (` ` :type "Actor Object Reference"))
  (returns (`  ` :type Boolean))
  (return false))

(fn `IsPlayerStatePlayerControlled`
  (params (PlayerState :type "PlayerState Object Reference"))
  (returns (bReturnValue :type Boolean))
  (return false))

(fn `IsShoveAttack`
  (params (DamageTakenEvent :type "DamageTakenEvent Structure (by ref)"))
  (returns (` ` :type Boolean))
  (return false))

(fn `IsTackleAttack`
  (params (DamageTakenEvent :type "DamageTakenEvent Structure (by ref)"))
  (returns (` ` :type Boolean))
  (return false))

(fn `TBLApplyCrowdControl`
  (params (DamageTaker :type "Actor Object Reference") (DamageCauser :type "Actor Object Reference") (CombatState :type "ECrowdControlCombatState Enum" :default "Interrupt") (CrowdControlParams :type "CrowdControlParams Structure") (bAutonomous :type Boolean)))

(fn `TBLApplyDamageAndCrowdControl`
  (params (DamageTaker :type "Actor Object Reference") (DamageCauser :type "Actor Object Reference") (Amount :type "Float (double-precision)") (DamageSource :type "DamageSource Object Reference") (CrowdControl :type Boolean) (CombatState :type "ECrowdControlCombatState Enum" :default "Interrupt") (CrowdControlParams :type "CrowdControlParams Structure") (bAutonomous :type Boolean) (InventoryItemOverride :type "InventoryItem Object Reference") (bOverrideImpactPoint :type Boolean) (DamageSourceLocationOverride :type "Vector Structure") (DamageInstigator :type "Actor Object Reference")))

(fn `TBLApplySphereDamageAndCC`
  (params (DamageCauser :type "Actor Object Reference") (Location :type "Vector Structure") (Radius :type "Float (double-precision)") (Amount :type "Float (double-precision)") (DamageSource :type "DamageSource Object Reference") (CrowdControl :type Boolean) (CombatState :type "ECrowdControlCombatState Enum" :default "Interrupt") (CrowdControlParams :type "CrowdControlParams Structure") (ActorsToIgnore :type "Array of Actor Object Reference (by ref)") (IgnoreSelf :type Boolean) (NoDamageCauserForAllies :type Boolean) (bOverrideImpactPoint :type Boolean)))

(fn `TBLGetActorsInSphere`
  (params (SpherePos :type "Vector Structure") (SphereRadius :type "Float (double-precision)") (DebugDraw :type Boolean))
  (returns (OutActors :type "Array of Actor Object Reference") (ReturnValue :type Boolean))
  (return _ false))

(fn `TBLKillPawn`
  (params (DamageTaker :type "Actor Object Reference") (DamageCauser :type "Actor Object Reference")))